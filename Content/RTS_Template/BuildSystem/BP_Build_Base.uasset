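; Base RTS building actor, configured from DT_BuildsData, covering placement, construction, worker assignment and removal.
; Placement snaps a green/red preview to the grid or a tagged resource node, then checks and deducts costs through GAS.
; Construction summons a free AI worker, then advances staged meshes on a timer with a progress widget.
; Completion applies gameplay effects to player and building; removal clears player effects and refunds half the wood, metal and scrap.
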(event Custom|On%20Build%20Starting%20Progress
  (bind _build_row (Variables|BuildInfo|GetBuild%20Row))
  ;[0.15 0.15 0.15 0.5 75] Start Build Process
  (Components|StaticMesh|SetStaticMesh (Variables|Default|GetBuildMesh) (Utilities|Array|Get(acopy) (.buildmeshes _build_row)))
  (if (Variables|WorkingBuild|GetWorker%20Near%20Building)
    (bind _returnvalue (Utilities|Time|SetTimerbyEvent (EventDispatchers|CreateEvent :!event Custom|Build%20Iteration%20Implement) (/ (.buildtime _build_row) (Utilities|Array|Length (.buildmeshes _build_row))) true))
    (Variables|BuildProgress|SetBuild%20Handler _returnvalue)
    (bind _returnvalue_2 (UserInterface|CreateWidget "/Game/RTS_Template/UI/Builds/WB_ProgressBuilding.WB_ProgressBuilding_C" 0 (.buildtime _build_row)))
    (UserInterface|SetWidget (Variables|Default|GetWidget) _returnvalue_2)
    (EventDispatchers|BindEventtoTimerEnded _returnvalue_2 (delegate Custom|Remove%20Widget%20Component))
    (else
      (CallFunction|WaitWorker))))

(event Custom|Build%20Iteration%20Implement
  (bind _build_row (Variables|BuildInfo|GetBuild%20Row))
  ;[0.15 0.15 0.15 0.5 45] BUILDING PROCESS
  (if (>= (Variables|BuildProgress|GetBuild%20Status%20Index) (Utilities|Array|LastIndex (.buildmeshes _build_row)))
    (CallFunction|FinishBuild)
    (else
      (bind _result (Math|Integer|IncrementInt (Variables|BuildProgress|GetBuild%20Status%20Index))
        (:%20%20
          (if (not (== _result (Utilities|Array|LastIndex (.buildmeshes _build_row))))
            (Components|StaticMesh|SetStaticMesh (Variables|Default|GetBuildMesh) (Utilities|Array|Get(acopy) (.buildmeshes _build_row) _result))
            (if (> (Variables|BuildProgress|GetBuild%20Status%20Index) (- (Utilities|Array|LastIndex (.buildmeshes _build_row)) 1))
              (CallFunction|FinishBuild))))))))

(event Custom|Wait%20Worker
  ;[0.15 0.15 0.15 0.5 45] FIND FREE WORKER
  (bind _returnvalue (Utilities|Time|SetTimerbyEvent (EventDispatchers|CreateEvent :!event Custom|Impl%20Check%20Worker) 1.0 true))
  (Variables|WorkingBuild|SetCheck%20Worker%20Handler _returnvalue))

(event Custom|Finish%20Build
  (bind _build_row (Variables|BuildInfo|GetBuild%20Row))
  ;[0.15 0.15 0.15 0.5 45] BUILDING PROCESS
  (Variables|Gameplay|SetBuilded true)
  (Utilities|Time|ClearandInvalidateTimerbyHandle (Variables|BuildProgress|GetBuild%20Handler))
  (Actor|Tick|SetActorTickEnabled true)
  (Components|StaticMesh|SetStaticMesh (Variables|Default|GetBuildMesh) (Utilities|Array|Get(acopy) (.buildmeshes _build_row) (Utilities|Array|LastIndex (.buildmeshes _build_row))))
  (Class|BPIAIBaseFace|StopWorkingBPI(Message) (Variables|WorkingBuild|GetWorker))
  (Variables|WorkingBuild|SetWorker 0)
  (GAS|ApplyResourceGameplayEffect)
  (GAS|StartGameplayEffects)
  (Default|CallWasBuilded))

(event Custom|Remove%20Widget%20Component
  ;[0.15 0.15 0.15 0.5 75] Start Build Process
  (UserInterface|SetWidget (Variables|Default|GetWidget) 0))

(event Custom|Impl%20Check%20Worker
  ;[0.15 0.15 0.15 0.5 45] FIND FREE WORKER
  (bind (_found_and_apply _founded_actor) (AI|LoopAIforWork))
  (if _found_and_apply
    (bind _output_get (Variables|WorkingBuild|SetWorker _founded_actor))
    (Class|BPIAIBaseFace|CalltoWorkBPI(Message) _output_get self)
    (Utilities|Time|ClearandInvalidateTimerbyHandle (Variables|WorkingBuild|GetCheck%20Worker%20Handler))
    (bind _returnvalue (Utilities|Time|SetTimerbyEvent (delegate Custom|Check%20Near%20Worker) 1.0 true))
    (Variables|WorkingBuild|SetCheck%20Near%20Worker%20Handler _returnvalue)))

(event Custom|Check%20Near%20Worker
  ;[0.15 0.15 0.15 0.5 45] FIND FREE WORKER
  (if (< (Math|Vector|Distance(Vector) (Transformation|GetActorLocation) (Transformation|GetActorLocation (Variables|WorkingBuild|GetWorker))) 9e+02)
    (Utilities|Time|ClearandInvalidateTimerbyHandle (Variables|WorkingBuild|GetCheck%20Near%20Worker%20Handler))
    (Variables|WorkingBuild|SetWorker%20Near%20Building true)
    (Default|CallBuildStartProgresstoBuild)))

(event Custom|Remove%20Building
  (GAS|RemoveAllGameplayEffects)
  (BUILDING|ReturnResources)
  (Actor|DestroyActor))

(event EventBeginPlay
  ;[0.15 0.15 0.15 0.5 45] Building Info APPLY
  (bind _returnvalue (Utilities|GetDataTableRow "/Game/RTS_Template/Data/DT_BuildsData.DT_BuildsData" (Variables|BuildInfo|GetBuilding%20Name))
    (:then
      (bind _output_get (Variables|BuildInfo|SetBuild%20Row _returnvalue))
      (Components|StaticMesh|SetStaticMesh (Variables|Default|GetBuildMesh) (Utilities|Array|Get(acopy) (.BuildMeshes (Utilities|Struct|BreakST_BuildInfoData _output_get)) (Utilities|Array|LastIndex (.BuildMeshes (Utilities|Struct|BreakST_BuildInfoData _output_get)))))
      (Collision|SetCollisionEnabled (Variables|Default|GetBuildMesh) (select (Variables|Gameplay|GetBuilded) "QueryAndPhysics" "NoCollision"))
      (Rendering|Material|SetMaterial (Variables|Default|GetBuildMesh) 0 (select (Variables|Gameplay|GetBuilded) (Variables|BuildInfo|GetBuilding%20Material) "/Game/RTS_Template/Materials/MI_OpacityRed.MI_OpacityRed"))
      (EventDispatchers|BindEventtoBuildStartProgresstoBuild (EventDispatchers|CreateEvent :!event Custom|On%20Build%20Starting%20Progress))
      (if (Variables|Gameplay|GetBuilded)
        ;[0.15 0.15 0.15 0.5] Start Gameplay Effects In Build
        (Variables|Components|GetPlayer%20Controller
          (:then
            _)
          (:else
            (Variables|Components|SetPlayer%20Controller (Game|GetPlayerController 0))))
        (GAS|StartGameplayEffects)
        (else
          ;[0.15 0.15 0.15 0.5] Check - Can Build per Place on World
          (bind _can (BUILDING|CanBuildThis? (Variables|Components|GetPlayer%20Controller) (Variables|BuildInfo|GetBuilding%20Name)))
          (if (not _can)
            (Actor|DestroyActor)))))))

(event Collision|EventActorBeginOverlap
  (params (OtherActor :type Actor%20Object%20Reference)))

(event EventTick
  (params (DeltaSeconds :type Float%20%28single-precision%29))
  (CallFunction|Debug)
  (switch Utilities|FlowControl|Switch|SwitchonEN_BuildingState (Variables|Gameplay|GetBuild%20State)
    (:NewEnumerator0
      (switch Utilities|FlowControl|Switch|SwitchonEN_BuildType (Variables|BuildType|GetBuild%20Type)
        (:NewEnumerator0
          (BUILDING|TraceandPlacePerBUILD))
        (:NewEnumerator1
          (BUILDING|TraceResourcePerBUILD))))))

(event EventBPIRotateBuild
  (bind _returnvalue (Transformation|GetActorRotation))
  ;[0.15 0.15 0.15 0.5] Rotate Building
  (Transformation|SetActorRotation (Math|Rotator|MakeRotator (.roll _returnvalue) (.pitch _returnvalue) (+ (.yaw _returnvalue) 45.0))))

(fn ConstructionScript)

(fn LineTraceStart-End
  (bind _returnvalue (Game|GetPlayerController 0))
  (bind _returnvalue_2 (Viewport|GetViewportSize))
  (bind _returnvalue_3 (/ (.y _returnvalue_2) 2.0))
  (bind _returnvalue_4 (/ (.x _returnvalue_2) 2.0))
  (bind _worldposition (Class|GameplayStatics|DeprojectScreentoWorld _returnvalue (Math|Vector2D|MakeVector2D _returnvalue_4 _returnvalue_3)))
  (return _worldposition (+ _worldposition (* (Math|Vector|GetForwardVector (Camera|GetCameraRotation (Game|GetPlayerCameraManager 0))) 9e+03))))

(fn GetHitResultbyInput
  (bind (_start _end) (Technical|LineTraceStart-End))
  (if (Variables|/Script/Engine.PlayerController|GetbShowMouseCursor (Variables|Components|GetPlayer%20Controller))
    (return (.HitResult (Game|Player|GetHitResultUnderCursorbyChannel (Variables|Components|GetPlayer%20Controller) "TraceTypeQuery2" true)))
    (else
      (bind _outhit (Collision|LineTraceByChannel _start _end "TraceTypeQuery1" false 0 "None"))
      (return _outhit))))

(fn TraceandPlacePerBUILD
  (if (not (Variables|Gameplay|GetBuilded))
    (Variables|Components|GetPlayer%20Controller
      (:then
        (bind _hitresult (Technical|GetHitResultbyInput))
        (if (.bBlockingHit (Collision|BreakHitResult _hitresult))
          (Transformation|SetActorLocation (Default|GetGridLocation (Variables|Default|GetBPC_Grid) (Math|Vector|MakeVector (.X (Math|Vector|BreakVector (.Location (Collision|BreakHitResult _hitresult)))) (.Y (Math|Vector|BreakVector (.Location (Collision|BreakHitResult _hitresult)))) (.Z (Math|Vector|BreakVector (.Location (Collision|BreakHitResult _hitresult)))))) false false)
          (bind _returnvalue (Collision|BoxTraceByChannel (+ (Default|GetGridLocation (Variables|Default|GetBPC_Grid) (Math|Vector|MakeVector (.X (Math|Vector|BreakVector (.Location (Collision|BreakHitResult _hitresult)))) (.Y (Math|Vector|BreakVector (.Location (Collision|BreakHitResult _hitresult)))) (.Z (Math|Vector|BreakVector (.Location (Collision|BreakHitResult _hitresult)))))) "0.000000,0.000000,950.000000") (+ (Default|GetGridLocation (Variables|Default|GetBPC_Grid) (Math|Vector|MakeVector (.X (Math|Vector|BreakVector (.Location (Collision|BreakHitResult _hitresult)))) (.Y (Math|Vector|BreakVector (.Location (Collision|BreakHitResult _hitresult)))) (.Z (Math|Vector|BreakVector (.Location (Collision|BreakHitResult _hitresult)))))) "0.000000,0.000000,950.000000") (Variables|Gameplay|GetProbe%20Half%20Size) (Transformation|GetActorRotation) "TraceTypeQuery1" true 0 "None"))
          (bind _output_get (Variables|Gameplay|SetCan%20Build (not _returnvalue)))
          (Rendering|Material|SetMaterial (Variables|Default|GetBuildMesh) 0 (select _output_get "/Game/RTS_Template/Materials/MI_OpacityGreen.MI_OpacityGreen" "/Game/RTS_Template/Materials/MI_OpacityRed.MI_OpacityRed"))))
      (:else))))

(fn TraceResourcePerBUILD
  (if (not (Variables|Gameplay|GetBuilded))
    (Variables|Components|GetPlayer%20Controller
      (:then
        (bind _hitresult (Technical|GetHitResultbyInput))
        (if (.bBlockingHit (Collision|BreakHitResult _hitresult))
          (Transformation|SetActorLocation (Default|GetGridLocation (Variables|Default|GetBPC_Grid) (Math|Vector|MakeVector (.X (Math|Vector|BreakVector (.Location (Collision|BreakHitResult _hitresult)))) (.Y (Math|Vector|BreakVector (.Location (Collision|BreakHitResult _hitresult)))) (.Z (Math|Vector|BreakVector (.Location (Collision|BreakHitResult _hitresult)))))) false false)
          (bind _output_get (Variables|Gameplay|SetCan%20Build (Actor|ActorHasTag (.HitActor (Collision|BreakHitResult _hitresult)) (Variables|BuildType|GetResource%20Tag))))
          (if _output_get
            (Transformation|SetActorTransform (Transformation|GetActorTransform (.HitActor (Collision|BreakHitResult _hitresult))))
            (Rendering|Material|SetMaterial (Variables|Default|GetBuildMesh) 0 "/Game/RTS_Template/Materials/MI_OpacityGreen.MI_OpacityGreen")
            (Variables|Gameplay|SetCan%20Build true)
            (Variables|BuildProgress|SetResource%20Object (.HitActor (Collision|BreakHitResult _hitresult)))
            (else
              (Rendering|Material|SetMaterial (Variables|Default|GetBuildMesh) 0 "/Game/RTS_Template/Materials/MI_OpacityRed.MI_OpacityRed")
              (Variables|Gameplay|SetCan%20Build false)))))
      (:else))))

(fn Debug
  (switch Utilities|FlowControl|Switch|SwitchonEN_BuildType (Variables|BuildType|GetBuild%20Type)))

(fn LoopAIforWork
  (bind _outactors (Actor|GetAllActorswithTag "AI"))
  (bind _array_element (Utilities|Array|ForEachLoopwithBreak _outactors :!label _label)
    (:LoopBody
      (bind _free_walked (Class|BPIAIBaseFace|AIIsFreeBPI(Message) _array_element))
      (if _free_walked
        (LocalVariables|SetLocal%20Found true)
        (LocalVariables|SetLocal%20Founded%20Worker _array_element)
        (goto _label Break)))
    (:Completed
      (return (LocalVariables|GetLocal%20Found) (LocalVariables|GetLocal%20Founded%20Worker)))))

(fn CanBuildThis?
  (params (GAS%20Owner :type Actor%20Object%20Reference) (Building%20Name :type Name))
  (LocalVariables|SetLocal%20Owner GAS%20Owner)
  (bind _returnvalue (Utilities|GetDataTableRow "/Game/RTS_Template/Data/DT_BuildsData.DT_BuildsData" Building%20Name)
    (:then
      (LocalVariables|SetLocal%20Cost (.Cost (Utilities|Struct|BreakST_BuildInfoData _returnvalue)))
      ;[0.15 0.15 0.15 0.5] Check Wood
      (if (>= (.ReturnValue (Ability|Attribute|GetFloatAttribute (LocalVariables|GetLocal%20Owner) "(AttributeName=\"Wood\",Attribute=/Script/Courpse.WC_AttributeSet:Wood,AttributeOwner=\"/Script/CoreUObject.Class'/Script/Courpse.WC_AttributeSet'\")")) (.wood (LocalVariables|GetLocal%20Cost)))
        ;[0.15 0.15 0.15 0.5] Check Metall
        (if (>= (.ReturnValue (Ability|Attribute|GetFloatAttribute (LocalVariables|GetLocal%20Owner) "(AttributeName=\"Metal\",Attribute=/Script/Courpse.WC_AttributeSet:Metal,AttributeOwner=\"/Script/CoreUObject.Class'/Script/Courpse.WC_AttributeSet'\")")) (.metal (LocalVariables|GetLocal%20Cost)))
          ;[0.15 0.15 0.15 0.5] Check Scrap
          (if (>= (.ReturnValue (Ability|Attribute|GetFloatAttribute (LocalVariables|GetLocal%20Owner) "(AttributeName=\"Scrap\",Attribute=/Script/Courpse.WC_AttributeSet:Scrap,AttributeOwner=\"/Script/CoreUObject.Class'/Script/Courpse.WC_AttributeSet'\")")) (.scrap (LocalVariables|GetLocal%20Cost)))
            ;[0.15 0.15 0.15 0.5] Check Technology
            (if (>= (.ReturnValue (Ability|Attribute|GetFloatAttribute (LocalVariables|GetLocal%20Owner) "(AttributeName=\"Technology\",Attribute=/Script/Courpse.WC_AttributeSet:Technology,AttributeOwner=\"/Script/CoreUObject.Class'/Script/Courpse.WC_AttributeSet'\")")) (.technology (LocalVariables|GetLocal%20Cost)))
              ;[0.15 0.15 0.15 0.5] Check Religion
              (if (>= (.ReturnValue (Ability|Attribute|GetFloatAttribute (LocalVariables|GetLocal%20Owner) "(AttributeName=\"Technology\",Attribute=/Script/Courpse.WC_AttributeSet:Technology,AttributeOwner=\"/Script/CoreUObject.Class'/Script/Courpse.WC_AttributeSet'\")")) (.technology (LocalVariables|GetLocal%20Cost)))
                (return true)
                (else
                  (return false)))
              (else
                (return false)))
            (else
              (return false)))
          (else
            (return false)))
        (else
          (return false))))
    (:RowNotFound
      (return false))))

(fn ThrowResources
  (LocalVariables|SetLocal%20Cost (.cost (Variables|BuildInfo|GetBuild%20Row)))
  (GAS|GASThrowRes "(TagName=\"Resources.Base.Wood\")" (.wood (LocalVariables|GetLocal%20Cost)))
  (GAS|GASThrowRes "(TagName=\"Resources.Base.Metal\")" (.metal (LocalVariables|GetLocal%20Cost)))
  (GAS|GASThrowRes "(TagName=\"Resources.Base.Scrap\")" (.scrap (LocalVariables|GetLocal%20Cost)))
  (GAS|GASThrowRes "(TagName=\"Resources.Base.Technology\")" (.technology (LocalVariables|GetLocal%20Cost)))
  (GAS|GASThrowRes "(TagName=\"Resources.Base.Religion\")" (.religion (LocalVariables|GetLocal%20Cost))))

(fn GASThrowRes
  (params (DataTag :type Gameplay%20Tag%20Structure) (Magnitude :type Float%20%28single-precision%29))
  (bind _player_controller (Variables|Components|GetPlayer%20Controller))
  (bind _returnvalue (Ability|GetAbilitySystemComponent _player_controller))
  (bind _returnvalue_2 (Ability|GameplayEffect|AssignTagSetbyCallerMagnitude (GameplayEffects|MakeOutgoingSpec :self _returnvalue :GameplayEffectClass "/Game/RTS_Template/GAS/Effects/GF_AddingStats.GF_AddingStats_C" :Level 1.0) DataTag (* Magnitude -1.0)))
  (GameplayEffects|ApplyGameplayEffectSpecToSelf _returnvalue _returnvalue_2))

(fn StartGameplayEffects
  (GAS|RemoveAllGameplayEffects)
  (bind _output_get (LocalVariables|SetLocal%20Effects (.gameplayeffects (Variables|BuildInfo|GetBuild%20Row))))
  (if (> (Utilities|Array|Length _output_get) 0)
    (LocalVariables|SetLocal%20Effect%20Level 5.0)
    ;[0.15 0.15 0.15 0.5] Player Effects
    (for _array_element (LocalVariables|GetLocal%20Effects)
      (bind _returnvalue (GameplayEffects|ApplyGameplayEffectToSelf :self (Ability|GetAbilitySystemComponent (Variables|Components|GetPlayer%20Controller)) :GameplayEffectClass _array_element :Level (LocalVariables|GetLocal%20Effect%20Level)))
      (Utilities|Array|Add (Variables|BuildInfo|GetBuilding%20Effects) _returnvalue))
    ;[0.15 0.15 0.15 0.5] Building Effects
    (for _array_element_2 (.selfeffects (Variables|BuildInfo|GetBuild%20Row))
      (GameplayEffects|ApplyGameplayEffectToSelf :self (Ability|GetAbilitySystemComponent self) :GameplayEffectClass _array_element_2 :Level (LocalVariables|GetLocal%20Effect%20Level)))))

(fn RemoveAllGameplayEffects
  (for _array_element (Variables|BuildInfo|GetBuilding%20Effects)
    (GameplayEffects|RemoveActiveGameplayEffect (Ability|GetAbilitySystemComponent (Variables|Components|GetPlayer%20Controller)) _array_element -1)))

(fn ReturnResources
  (LocalVariables|SetLocal%20Cost (.cost (Variables|BuildInfo|GetBuild%20Row)))
  (GAS|GASThrowRes "(TagName=\"Resources.Base.Wood\")" (BUILDING|CheckReturnValue (.wood (LocalVariables|GetLocal%20Cost))))
  (GAS|GASThrowRes "(TagName=\"Resources.Base.Metal\")" (BUILDING|CheckReturnValue (.metal (LocalVariables|GetLocal%20Cost))))
  (GAS|GASThrowRes "(TagName=\"Resources.Base.Scrap\")" (BUILDING|CheckReturnValue (.scrap (LocalVariables|GetLocal%20Cost)))))

(fn CheckReturnValue
  (params (Value :type Float%20%28double-precision%29))
  (if (<= Value 0.0)
    (return 0.0)
    (else
      (return (* (/ Value 2.0) -1.0)))))

(fn ApplyResourceGameplayEffect
  (bind _cppabilitysystemcomponent (Variables|Default|GetCppAbilitySystemComponent))
  (bind _build_row (Variables|BuildInfo|GetBuild%20Row))
  (if (or (> (.resourcelimit _build_row) 0.0) (> (Variables|Resource|GetResource%20Limit) 0.0))
    (bind _output_get (LocalVariables|SetLocal%20Resourse (select (<= (Variables|Resource|GetResource%20Limit) 0.0) (.resourcelimit _build_row) (Variables|Resource|GetResource%20Limit))))
    (bind _returnvalue (Ability|GameplayEffect|AssignTagSetbyCallerMagnitude (GameplayEffects|MakeOutgoingSpec :self _cppabilitysystemcomponent :GameplayEffectClass "/Game/RTS_Template/BuildSystem/Gas/BaseEffects/BGE_InstantResource.BGE_InstantResource_C" :Level 1.0) "(TagName=\"Building.Resource\")" _output_get))
    (GameplayEffects|ApplyGameplayEffectSpecToSelf _cppabilitysystemcomponent _returnvalue)))

(fn BPIAddWorker
  (params (AI%20Worker :type Actor%20Object%20Reference))
  (Utilities|IsValid AI%20Worker
    (:Is%20Valid
      (LocalVariables|SetLocal%20Worker%20Actor AI%20Worker)
      (if (>= (Utilities|Array|Length (Variables|WorkProgress|GetWorkers%20Progress)) (.maxworkers (Variables|BuildInfo|GetBuild%20Row)))
        (return false)
        (else
          (Utilities|Array|Add (Variables|WorkProgress|GetWorkers%20Progress) (LocalVariables|GetLocal%20Worker%20Actor))
          (Class|BPIAIBaseFace|AddWorkingtoBuildingBPI(Message) (LocalVariables|GetLocal%20Worker%20Actor) self)
          (Default|CallWorkerChanged)
          (return true))))
    (:Is%20Not%20Valid
      (return false))))

(fn BPIBuildStart
  (if (Variables|Gameplay|GetCan%20Build)
    (bind _can (BUILDING|CanBuildThis? (Variables|Components|GetPlayer%20Controller) (Variables|BuildInfo|GetBuilding%20Name)))
    (if _can
      (switch Utilities|FlowControl|Switch|SwitchonEN_BuildingState (Variables|Gameplay|GetBuild%20State)
        (:NewEnumerator0
          (Rendering|Material|SetMaterial (Variables|Default|GetBuildMesh) 0 (Variables|BuildInfo|GetBuilding%20Material))
          (Collision|SetCollisionEnabled (Variables|Default|GetBuildMesh) "QueryAndPhysics")
          (CameraShakes|StartCameraShake (Variables|/Script/Engine.PlayerController|GetPlayerCameraManager (Variables|Components|GetPlayer%20Controller)) "/Game/CameraShakes/Legacy/LCS_FireDefault.LCS_FireDefault_C" 1.0 "CameraLocal" "0, 0, 0")
          (Variables|Gameplay|SetBuild%20State "NewEnumerator1")
          (Default|CallBuildStartProgresstoBuild)
          (bind _resource_object (Variables|BuildProgress|GetResource%20Object)
            (:then
              ;[0.15 0.15 0.15 0.5] Resource Limits And Off Collision
              (bind _resource_limit (Class|BPIBuilding|BPIGetResourceLimit(Message) _resource_object))
              (Variables|Resource|SetResource%20Limit _resource_limit)
              (Collision|SetActorEnableCollision _resource_object false))
            (:else
              _))
          (BUILDING|ThrowResources)
          (return true))
        (:NewEnumerator1
          _)
        (:NewEnumerator2
          _))
      (return false))))

(fn BPICanCheckBuild
  (Utilities|GetDataTableRow "/Game/RTS_Template/Data/DT_BuildsData.DT_BuildsData" (Variables|BuildInfo|GetBuilding%20Name)
    (:then
      (return true))
    (:RowNotFound
      (return false))))

(fn BPIGetBuildInteract
  (return self))

(fn BPIGetResourceLimit
  (return (Variables|Resource|GetResource%20Limit)))

(fn BPIGetWorkersAmount
  (return (Utilities|Array|Length (Variables|WorkProgress|GetWorkers%20Progress))))

(fn BPIRemoveWorker
  (if (> (Utilities|Array|Length (Variables|WorkProgress|GetWorkers%20Progress)) 0)
    (bind _output_get (LocalVariables|SetLocal%20Found%20Worker (.OutItem (Utilities|Array|Random (Variables|WorkProgress|GetWorkers%20Progress)))))
    (Class|BPIAIBaseFace|StopWorkingBPI(Message) _output_get)
    (Utilities|Array|RemoveItem (Variables|WorkProgress|GetWorkers%20Progress) (LocalVariables|GetLocal%20Found%20Worker))
    (Default|CallWorkerChanged)
    (return true)
    (else
      (return false))))