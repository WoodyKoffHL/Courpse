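; RTS camera pawn that handles panning, screen-edge scrolling, zoom and yaw rotation.
; Enhanced Input drives movement along actor axes, clamped spring-arm length for zoom, and world yaw.
; A "Movement Mouse XY" graph turns cursor position near viewport edges into speeds, applied as local offsets.
; The fast-move input raises pawn max speed and a sensitivity multiplier shared by edge scrolling, zoom and rotation.
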(event Input|EnhancedActionEvents|EnhancedInputActionIA_RTS_CameraMoving
  (params (ActionValue :type Vector%202D%20Structure) (ElapsedSeconds :type Float%20%28double-precision%29) (TriggeredSeconds :type Float%20%28double-precision%29) (InputAction :type Input%20Action%20Object%20Reference :default "/Game/RTS_Template/Input/IA_RTS_CameraMoving.IA_RTS_CameraMoving"))
  (bind (_x _y) (Math|Vector2D|BreakVector2D ActionValue))
  ;[0.15 0.15 0.15 0.5] Camera Manual Move
  (Pawn|Input|AddMovementInput (Transformation|GetActorForwardVector) _y false)
  (Pawn|Input|AddMovementInput (Transformation|GetActorRightVector) _x false))

(event Input|EnhancedActionEvents|EnhancedInputActionIA_RTS_FastMoving
  (params (ActionValue :type Boolean) (ElapsedSeconds :type Float%20%28double-precision%29) (TriggeredSeconds :type Float%20%28double-precision%29) (InputAction :type Input%20Action%20Object%20Reference :default "/Game/RTS_Template/Input/IA_RTS_FastMoving.IA_RTS_FastMoving"))
  (bind _floatingpawnmovement (Variables|Default|GetFloatingPawnMovement))
  ;[0.15 0.15 0.15 0.5] Camera Manual Move
  (:Started
    (Variables|/Script/Engine.FloatingPawnMovement|SetMaxSpeed _floatingpawnmovement 6e+03)
    (Variables|Default|SetMove%20Sens 2.0))
  (:Completed
    (Variables|/Script/Engine.FloatingPawnMovement|SetMaxSpeed _floatingpawnmovement 3e+03)
    (Variables|Default|SetMove%20Sens 1.0)))

(event Input|EnhancedActionEvents|EnhancedInputActionIA_RTS_Zoom
  (params (ActionValue :type Float%20%28double-precision%29) (ElapsedSeconds :type Float%20%28double-precision%29) (TriggeredSeconds :type Float%20%28double-precision%29) (InputAction :type Input%20Action%20Object%20Reference :default "/Game/RTS_Template/Input/IA_RTS_Zoom.IA_RTS_Zoom"))
  (bind _springarm (Variables|Default|GetSpringArm))
  ;[0.15 0.15 0.15 0.5] Zoom
  (Variables|/Script/Engine.SpringArmComponent|SetTargetArmLength _springarm (Math|Float|Clamp(Float) (+ (Variables|/Script/Engine.SpringArmComponent|GetTargetArmLength _springarm) (* (select (> ActionValue 0.6) -5e+01 5e+01) (Variables|Default|GetMove%20Sens))) 0.0 4e+03)))

(event Input|EnhancedActionEvents|EnhancedInputActionIA_RTS_Rotate
  (params (ActionValue :type Float%20%28double-precision%29) (ElapsedSeconds :type Float%20%28double-precision%29) (TriggeredSeconds :type Float%20%28double-precision%29) (InputAction :type Input%20Action%20Object%20Reference :default "/Game/RTS_Template/Input/IA_RTS_Rotate.IA_RTS_Rotate"))
  (Class|Actor|AddActorWorldRotation (Math|Rotator|MakeRotator 0.0 0.0 (* ActionValue (Variables|Default|GetMove%20Sens)))))

(event EventBeginPlay)

(event Collision|EventActorBeginOverlap
  (params (OtherActor :type Actor%20Object%20Reference)))

(event EventTick
  (params (DeltaSeconds :type Float%20%28single-precision%29)))

(event Input|MouseEvents|MouseX
  (params (AxisValue :type Float%20%28single-precision%29))
  (bind _move_sens (Variables|Default|GetMove%20Sens))
  ;[0.15 0.15 0.15 0.5] Camera Manual Move
  (bind (_speed_x _speed_y) (Utilities|MovementMouseXY)
    (:Return
      (Transformation|AddActorLocalOffset (Math|Vector|MakeVector (* _speed_x 3.0 _move_sens) (* _speed_y 3.0 _move_sens) 0.0) false false))))

(event Input|MouseEvents|MouseY
  (params (AxisValue :type Float%20%28single-precision%29))
  (bind _move_sens (Variables|Default|GetMove%20Sens))
  ;[0.15 0.15 0.15 0.5] Camera Manual Move
  (Utilities|MovementMouseXY) ; enters at Move Y
)

(fn ConstructionScript)