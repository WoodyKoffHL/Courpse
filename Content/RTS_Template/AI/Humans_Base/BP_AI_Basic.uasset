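; BP_AI_Basic is the base human AI worker for the RTS template, taking work and building orders through interface calls.
; On BeginPlay it spawns its controller, runs BT_Basic_Ai and seeds the blackboard with its state.
; Orders write a target location and change the AI state enum, whose RepNotify mirrors it to the blackboard.
; Stopping work restores the state that the availability check reports as free.
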(event EventBeginPlay
  (Pawn|SpawnDefaultController)
  (AI|RunBehaviorTree (AI|GetAIController self) "/Game/RTS_Template/AI/Blueprints/BT_Basic_Ai.BT_Basic_Ai")
  (AI|Components|Blackboard|SetValueasEnum (AI|GetBlackboard 0) (Utilities|Name|MakeLiteralName "EN_AIState") (Variables|Default|GetEN%20AI%20State)))

(event Collision|EventActorBeginOverlap
  (params (OtherActor :type Actor%20Object%20Reference)))

(event EventTick
  (params (DeltaSeconds :type Float%20%28single-precision%29)))

(event EventCalltoWorkBPI
  (params (Actor%20to%20Work :type Actor%20Object%20Reference))
  (CallFunction|SetTargetLocation (Transformation|GetActorLocation Actor%20to%20Work))
  (Variables|Default|SetEN%20AI%20State "NewEnumerator2"))

(event EventStopWorkingBPI
  (Variables|Default|SetEN%20AI%20State "NewEnumerator0"))

(event EventAddWorkingtoBuildingBPI
  (params (Building :type Actor%20Object%20Reference))
  (CallFunction|SetTargetLocation (Transformation|GetActorLocation Building))
  (Variables|Default|SetEN%20AI%20State "NewEnumerator3"))

(fn ConstructionScript)

(fn OnRepENAIState
  (AI|Components|Blackboard|SetValueasEnum (AI|GetBlackboard 0) (Utilities|Name|MakeLiteralName "EN_AIState") (Variables|Default|GetEN%20AI%20State)))

(fn SetTargetObject
  (params (ObjectValue :type Actor%20Object%20Reference))
  (AI|Components|Blackboard|SetValueasObject (AI|GetBlackboard 0) (Utilities|Name|MakeLiteralName "TargetObject") ObjectValue))

(fn SetTargetLocation
  (params (VectorValue :type Vector))
  (AI|Components|Blackboard|SetValueasVector (AI|GetBlackboard 0) (Utilities|Name|MakeLiteralName "TargetLocation") VectorValue))

(fn AIIsFreeBPI
  (return (Utilities|Enum|Equal(Enum) (Variables|Default|GetEN%20AI%20State) "NewEnumerator0")))