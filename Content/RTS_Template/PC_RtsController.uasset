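; RTS player controller that handles building placement, building selection and starting resources.
; Enhanced Input toggles the build menu or cancels placement, spawns the chosen building, then rotates or confirms it through interface messages.
; Clicking a qualifying building opens a single info widget, and GetHitResultByInput switches between cursor and screen-center traces as gamepad use toggles the cursor.
; GAS effects set starting stats and Wood, which Tick prints as debug text.
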(event Custom|Close%20Actibe%20Build%20Widget
  ;[0.15 0.15 0.15 0.5] Close Building Widget
  (Widget|RemovefromParent (Variables|UI|GetActive%20Build%20Widget))
  (Variables|UI|SetActive%20Build%20Widget 0))

(event Input|EnhancedActionEvents|EnhancedInputActionIA_RTS_StartBuild
  (params (ActionValue :type Boolean) (ElapsedSeconds :type Float%20%28double-precision%29) (TriggeredSeconds :type Float%20%28double-precision%29) (InputAction :type Input%20Action%20Object%20Reference :default "/Game/RTS_Template/Input/IA_RTS_StartBuild.IA_RTS_StartBuild"))
  ;[0.15 0.15 0.15 0.5] Button Start Build
  (:Started
    (CallFunction|StartBuildObject)))

(event Input|EnhancedActionEvents|EnhancedInputActionIA_RTS_LeftClick
  (params (ActionValue :type Boolean) (ElapsedSeconds :type Float%20%28double-precision%29) (TriggeredSeconds :type Float%20%28double-precision%29) (InputAction :type Input%20Action%20Object%20Reference :default "/Game/RTS_Template/Input/IA_RTS_LeftClick.IA_RTS_LeftClick"))
  ;[0.15 0.15 0.15 0.5] Left Click
  (:Started
    (Variables|Default|GetBuilding%20In%20Process
      (:then
        (bind _start_biuld (Class|BPIBuilding|BPIBuildStart(Message) (Variables|Default|GetBuilding%20In%20Process)))
        (if _start_biuld
          (Variables|Default|SetBuilding%20In%20Process 0)))
      (:else
        (CallFunction|ClickonWorld)))))

(event Input|EnhancedActionEvents|EnhancedInputActionIA_RTS_MiddleMouse
  (params (ActionValue :type Boolean) (ElapsedSeconds :type Float%20%28double-precision%29) (TriggeredSeconds :type Float%20%28double-precision%29) (InputAction :type Input%20Action%20Object%20Reference :default "/Game/RTS_Template/Input/IA_RTS_MiddleMouse.IA_RTS_MiddleMouse"))
  ;[0.15 0.15 0.15 0.5] Rotate Building
  (:Started
    (bind _building_in_process (Variables|Default|GetBuilding%20In%20Process)
      (:then
        (Class|BPIBuilding|BPIRotateBuild(Message) _building_in_process))
      (:else))))

(event EventBeginPlay
  ;[0.15 0.15 0.15 0.5] Input System
  (Input|AddMappingContext (PlayerController|LocalPlayerSubsystems|GetEnhancedInputLocalPlayerSubsystem self) "/Game/RTS_Template/Input/IMC_RTS.IMC_RTS" 0 (Utilities|Struct|MakeModifyContextOptions true false false))
  (CallFunction|CAStartGameGAS))

(event Input|KeyboardEvents|AnyKey
  (params (Key :type Key%20Structure :default "None"))
  ;[0.15 0.15 0.15 0.5] Check Gamepad
  (:Pressed
    (Variables|Default|SetbShowMouseCursor (not (Class|KismetInputLibrary|KeyIsGamepadKey Key)))))

(event Custom|Start%20Building
  (params (Object :type BP%20Build%20Base%20Class%20Reference))
  ;[0 0.05404 0.15 0.5 70] START BUILD OBJECT
  (if (Utilities|IsValidClass Object)
    (bind _returnvalue (Game|SpawnActorfromClass Object (Math|Transform|MakeTransform "0, 0, 0" "0, 0, 0" "1.000000,1.000000,1.000000") "Undefined" "MultiplyWithRoot" 0 self "NewEnumerator0" 0))
    (Variables|Default|SetBuilding%20In%20Process _returnvalue))
  (Widget|RemovefromParent (Variables|UI|GetUI%20Widget%20Buildings))
  (Variables|UI|SetUI%20Widget%20Buildings 0))

(event Custom|Start%20Build%20Object
  ;[0 0.05404 0.15 0.5 70] START BUILD OBJECT
  (bind _ui_widget_buildings (Variables|UI|GetUI%20Widget%20Buildings)
    (:then
      (Widget|RemovefromParent _ui_widget_buildings)
      (Variables|UI|SetUI%20Widget%20Buildings 0))
    (:else
      (Variables|Default|GetBuilding%20In%20Process
        (:then
          (Actor|DestroyActor (Variables|Default|GetBuilding%20In%20Process))
          (Variables|Default|SetBuilding%20In%20Process 0))
        (:else
          (bind _returnvalue (UserInterface|CreateWidget "/Game/RTS_Template/UI/WB_Buildings.WB_Buildings_C"))
          (bind _output_get (Variables|UI|SetUI%20Widget%20Buildings _returnvalue))
          (EventDispatchers|BindEventtoStartBuildObject _output_get (delegate Custom|Start%20Building))
          (UserInterface|Viewport|AddtoViewport (Variables|UI|GetUI%20Widget%20Buildings) 0))))))

(event EventTick
  (params (DeltaSeconds :type Float%20%28single-precision%29))
  (Development|PrintString (Utilities|String|Append (Utilities|String|Append "Wood: " (Utilities|String|Append (Utilities|String|ToString(Float) (.ReturnValue (Ability|Attribute|GetFloatAttribute self "(AttributeName=\"Wood\",Attribute=/Script/Courpse.WC_AttributeSet:Wood,AttributeOwner=\"/Script/CoreUObject.Class'/Script/Courpse.WC_AttributeSet'\")"))) "/" (Utilities|String|ToString(Float) (.ReturnValue (Ability|Attribute|GetFloatAttribute self "(AttributeName=\"MaxWood\",Attribute=/Script/Courpse.WC_AttributeSet:MaxWood,AttributeOwner=\"/Script/CoreUObject.Class'/Script/Courpse.WC_AttributeSet'\")"))))) " " "" " " "" " " "" " ") true true "(R=0.000000,G=0.660000,B=1.000000,A=1.000000)" 0.0))

(event Custom|CA%20Start%20Game%20GAS
  (GameplayEffects|ApplyGameplayEffectToSelf :self (Variables|Default|GetCppAbilitySystemComponent) :GameplayEffectClass "/Game/RTS_Template/GAS/Effects/GF_SetMaxStartStats.GF_SetMaxStartStats_C" :Level 1.0)
  (bind _returnvalue (Ability|GameplayEffect|AssignTagSetbyCallerMagnitude (GameplayEffects|MakeOutgoingSpec :self (Variables|Default|GetCppAbilitySystemComponent) :GameplayEffectClass "/Game/RTS_Template/GAS/Effects/GF_AddingStats.GF_AddingStats_C" :Level 1.0) "(TagName=\"Resources.Base.Wood\")" 2e+02))
  (GameplayEffects|ApplyGameplayEffectSpecToSelf (Variables|Default|GetCppAbilitySystemComponent) _returnvalue))

(event Input|KeyboardEvents|DebugKeyU
  (params (Key :type Key%20Structure :default "None") (ActionValue :type Input%20Action%20Value%20Structure)))

(fn ConstructionScript)

(fn GetHitResultbyInput
  (bind (_start _end) (CallFunction|LineTraceStart-End))
  (if (Variables|Default|GetbShowMouseCursor)
    (return (.HitResult (Game|Player|GetHitResultUnderCursorbyChannel "TraceTypeQuery2" true)))
    (else
      (bind _outhit (Collision|LineTraceByChannel _start _end "TraceTypeQuery1" false 0 "None"))
      (return _outhit))))

(fn LineTraceStart-End
  (bind _returnvalue (Viewport|GetViewportSize))
  (bind _self self)
  (bind _returnvalue_2 (/ (.y _returnvalue) 2.0))
  (bind _returnvalue_3 (/ (.x _returnvalue) 2.0))
  (bind _worldposition (Class|GameplayStatics|DeprojectScreentoWorld _self (Math|Vector2D|MakeVector2D _returnvalue_3 _returnvalue_2)))
  (return _worldposition (+ _worldposition (* (Math|Vector|GetForwardVector (Camera|GetCameraRotation (Game|GetPlayerCameraManager 0))) 9e+03))))

(fn ClickonWorld
  (bind _hitresult (Game|Player|GetHitResultUnderCursorbyChannel "TraceTypeQuery2" true))
  (if (Utilities|DoesObjectImplementInterface (.hitactor _hitresult) "/Game/RTS_Template/Components/BPI_BuildIngteracts.BPI_BuildIngteracts_C")
    (bind _can (Class|BPIBuildIngteracts|BPICanCheckBuild(Message) (.hitactor _hitresult)))
    (if _can
      (Variables|UI|GetActive%20Build%20Widget
        (:then
          (if (not (== (Variables|/Game/RTS_Template/UI/WB_BuildingInfo.WB_BuildingInfo_C|GetBuild%20Base (Variables|UI|GetActive%20Build%20Widget)) (.hitactor _hitresult)))
            (Widget|RemovefromParent (Variables|UI|GetActive%20Build%20Widget))
            (Variables|UI|SetActive%20Build%20Widget 0)
            (bind _active_build (Class|BPIBuildIngteracts|BPIGetBuildInteract(Message) (.hitactor _hitresult) :!label _label))
            (bind _returnvalue (UserInterface|CreateWidget "/Game/RTS_Template/UI/WB_BuildingInfo.WB_BuildingInfo_C" self _active_build))
            (bind _output_get (Variables|UI|SetActive%20Build%20Widget _returnvalue))
            (EventDispatchers|BindEventtoBuildWidgetClose _output_get (EventDispatchers|CreateEvent :!event Custom|Close%20Actibe%20Build%20Widget))
            (UserInterface|Viewport|AddtoViewport (Variables|UI|GetActive%20Build%20Widget) 0)))
        (:else
          (goto _label))))))